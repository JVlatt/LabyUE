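; Enemy patrol Blueprint that walks between two patrol points and chases the player on sight, restarting the current level when it reaches them.
; BeginPlay starts a recursive Patrol event using AI MoveTo to each point with a pause at both, looping while Vision is false.
; Pawn Sensing sets Vision on seeing a FirstPersonCharacter and moves toward it; nothing in the graph ever clears Vision.
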(event OnSeePawn(PawnSensing)
  (params (Pawn :type Pawn%20Object%20Reference))
  (Variables|Default|SetVision true)
  (bind _asfirst_person_character (Utilities|Casting|CastToFirstPersonCharacter Pawn))
  (AI|AIMoveTo self "0, 0, 0" _asfirst_person_character 5.0 false
    (:OnSuccess
      (bind _returnvalue (Game|GetCurrentLevelName true))
      (Game|OpenLevel(byName) (Utilities|String|StringToName _returnvalue)))))

(event Custom|Patrol
  (if (not (Variables|Default|GetVision))
    (AI|AIMoveTo self "0, 0, 0" (Variables|Default|GetPatrolPoint1) 5.0 false
      (:OnSuccess
        (Utilities|FlowControl|Delay 3.0)
        (AI|AIMoveTo self "0, 0, 0" (Variables|Default|GetPatrolPoint2) 5.0 false
          (:OnSuccess
            (Utilities|FlowControl|Delay 3.0)
            (CallFunction|Patrol)))))))

(event EventBeginPlay
  (CallFunction|Patrol))

(fn ConstructionScript)